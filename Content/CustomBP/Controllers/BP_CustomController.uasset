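; BP_CustomController is a player controller that drives movement and attacking for the controlled pawn, with the mouse cursor shown.
; Axis inputs add movement along the control rotation's forward and right vectors while no attack is active.
; The Attack action calls Attack on the pawn, cast to BP_CustomCharacter, and sets IsAttacking.
; A short timer clears that flag, which blocks movement but does not gate further attack presses.
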(event `self.ReceiveBeginPlay`)

(event `self.ReceiveTick`
  (params (DeltaSeconds :type "Float (single-precision)")))

(event `InputAxis|MoveHorizontally`
  (params (AxisValue :type "Float (single-precision)"))
  (bind _returnvalue (`self.K2_GetPawn`))
  (bind (_returnvalue_roll _returnvalue_pitch _returnvalue_yaw) (`KismetMathLibrary.BreakRotator` (`self.GetControlRotation` self)))
  (if (and (not (`self.isAttacking`)) (`KismetSystemLibrary.IsValid` _returnvalue))
    (`Pawn.AddMovementInput` _returnvalue (`KismetMathLibrary.GetRightVector` (`KismetMathLibrary.MakeRotator` _returnvalue_roll 0.0 _returnvalue_yaw)) AxisValue false)))

(event `InputAxis|MoveVertically`
  (params (AxisValue :type "Float (single-precision)"))
  (bind _returnvalue (`self.K2_GetPawn`))
  (bind (_returnvalue_roll _returnvalue_pitch _returnvalue_yaw) (`KismetMathLibrary.BreakRotator` (`self.GetControlRotation` self)))
  (if (and (not (`self.isAttacking`)) (`KismetSystemLibrary.IsValid` _returnvalue))
    (`Pawn.AddMovementInput` _returnvalue (`KismetMathLibrary.GetForwardVector` (`KismetMathLibrary.MakeRotator` 0.0 0.0 _returnvalue_yaw)) AxisValue false)))

(event `InputAction|Attack`
  (params (Key :type "Key Structure"))
  (:`Pressed`
    (bind _pawn (`self.GetPawnAsCharacter`))
    (`/Engine/EditorBlueprintResources/StandardMacros.IsValid` _pawn
      (:`Is Valid`
        (`/Game/CustomBP/Characters/BP_CustomCharacter.Attack` _pawn)
        (set `self.isAttacking` true)
        (`KismetSystemLibrary.K2_SetTimerDelegate` (delegate `AttackCooldown`) 0.6)))))

(event `AttackCooldown`
  (set `self.isAttacking` false))

(fn `GetPawnAsCharacter`
  (returns (pawn :type "/Game/CustomBP/Characters/BP_CustomCharacter Object Reference"))
  (locals (thisPawn :type "/Game/CustomBP/Characters/BP_CustomCharacter Object Reference"))
  (bind _returnvalue (`self.K2_GetPawn`))
  (bind (_asbp_custom_character _bsuccess) (cast `/Game/CustomBP/Characters/BP_CustomCharacter` _returnvalue :!pure true))
  (if (and (`KismetSystemLibrary.IsValid` _returnvalue) _bsuccess)
    (set `local.thisPawn` _asbp_custom_character))
  (return (`local.thisPawn`)))

(fn `UserConstructionScript`
  (set `self.bShowMouseCursor` true))