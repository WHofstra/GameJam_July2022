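; AI controller that drives enemy characters with a test behavior tree and blackboard.
; On BeginPlay it initializes the blackboard, stores the first player character under the player key, then runs the behavior tree.
; A helper function casts the controlled pawn to the enemy character class and returns it.
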(event `self.ReceiveBeginPlay`
  (bind _blackboardcomponent (`self.UseBlackboard` "/Game/CustomBP/AI/BB_TestBlackBoard.BB_TestBlackBoard"))
  (`BlackboardComponent.SetValueAsObject` _blackboardcomponent (`self.playerKey`) (`GameplayStatics.GetPlayerCharacter` 0))
  (`self.RunBehaviorTree` "/Game/CustomBP/AI/BT_TestBehaviourTree.BT_TestBehaviourTree"))

(event `self.ReceiveTick`
  (params (DeltaSeconds :type "Float (single-precision)")))

(fn `GetPawnAsEnemy`
  (returns (enemy :type "/Game/CustomBP/Characters/BP_EnemyCharacter Object Reference"))
  (locals (anEnemy :type "/Game/CustomBP/Characters/BP_EnemyCharacter Object Reference"))
  (bind _returnvalue (`self.K2_GetPawn`))
  (bind (_asbp_enemy_character _bsuccess) (cast `/Game/CustomBP/Characters/BP_EnemyCharacter` _returnvalue :!pure true))
  (if (and (`KismetSystemLibrary.IsValid` _returnvalue) _bsuccess)
    (set `local.anEnemy` _asbp_enemy_character))
  (return (`local.anEnemy`)))

(fn `UserConstructionScript`)