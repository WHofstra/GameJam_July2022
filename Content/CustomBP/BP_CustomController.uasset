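; Custom player controller that shows the mouse cursor and drives the controlled pawn's movement and jumping.
; Movement axes add input relative to control rotation, with MoveHorizontally using the yaw-only forward vector and MoveVertically the right vector from yaw and roll.
; Jump calls a GetPawnAsCharacter helper, which casts the pawn to Character and stores it in ThisPawn, then triggers Jump on the result if valid.
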(event `self.ReceiveBeginPlay`)

(event `self.ReceiveTick`
  (params (DeltaSeconds :type "Float (single-precision)")))

(event `InputAxis|MoveHorizontally`
  (params (AxisValue :type "Float (single-precision)"))
  (bind _returnvalue (`self.K2_GetPawn`))
  (bind (_returnvalue_roll _returnvalue_pitch _returnvalue_yaw) (`KismetMathLibrary.BreakRotator` (`self.GetControlRotation` self)))
  (if (`KismetSystemLibrary.IsValid` _returnvalue)
    (`Pawn.AddMovementInput` _returnvalue (`KismetMathLibrary.GetForwardVector` (`KismetMathLibrary.MakeRotator` 0.0 0.0 _returnvalue_yaw)) AxisValue false)))

(event `InputAxis|MoveVertically`
  (params (AxisValue :type "Float (single-precision)"))
  (bind _returnvalue (`self.K2_GetPawn`))
  (bind (_returnvalue_roll _returnvalue_pitch _returnvalue_yaw) (`KismetMathLibrary.BreakRotator` (`self.GetControlRotation` self)))
  (if (`KismetSystemLibrary.IsValid` _returnvalue)
    (`Pawn.AddMovementInput` _returnvalue (`KismetMathLibrary.GetRightVector` (`KismetMathLibrary.MakeRotator` _returnvalue_roll 0.0 _returnvalue_yaw)) AxisValue false)))

(event `InputAction|Jump`
  (params (Key :type "Key Structure"))
  (:`Pressed`
    (bind _pawn (`self.GetPawnAsCharacter`))
    (if (`KismetSystemLibrary.IsValid` _pawn)
      (`Character.Jump` _pawn))))

(fn `GetPawnAsCharacter`
  (returns (pawn :type "Character Object Reference"))
  (locals (thisPawn :type "Character Object Reference"))
  (bind _returnvalue (`self.K2_GetPawn`))
  (bind (_ascharacter _bsuccess) (cast `Character` _returnvalue :!pure true))
  (if (and (`KismetSystemLibrary.IsValid` _returnvalue) _bsuccess)
    (set `local.thisPawn` _ascharacter))
  (return (`local.thisPawn`)))

(fn `UserConstructionScript`
  (set `self.bShowMouseCursor` true))