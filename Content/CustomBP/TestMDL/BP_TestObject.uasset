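; BP_TestObject is a test actor with an availability flag and a static mesh whose physics simulation can be toggled.
; Functions read the flag, set it immediately, or pass a value and duration to a timer event.
; That event plays TimedCooldown and applies the value when it finishes, though the timed setter returns the new value right away.
; BeginPlay, Tick and overlap events are empty.
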(event `self.ReceiveBeginPlay`)

(event `self.ReceiveActorBeginOverlap`
  (params (OtherActor :type "Actor Object Reference")))

(event `self.ReceiveTick`
  (params (DeltaSeconds :type "Float (single-precision)")))

(event `SetTimerAvailability`
  (params (value :type Boolean) (seconds :type "Float (double-precision)"))
  (`Timeline|TimedCooldown` :`NewTime` seconds
    (:`Finished`
      (set `self.availability` value))))

(fn `IsAvailable`
  (returns (isAvailable :type Boolean))
  (return (`self.availability`)))

(fn `SetAvailabilityTo`
  (params (newValue :type Boolean))
  (returns (isAvailable :type Boolean))
  (bind _output_get (set `self.availability` newValue))
  (return _output_get))

(fn `SetAvailabilityWithTimer`
  (params (newValue :type Boolean) (seconds :type "Float (double-precision)"))
  (returns (isAvailable :type Boolean))
  (`self.SetTimerAvailability` newValue seconds)
  (return newValue))

(fn `SimulatePhysics`
  (params (simulate :type Boolean))
  (returns (isSet :type Boolean))
  (`PrimitiveComponent.SetSimulatePhysics` (`self.StaticMesh`) simulate)
  (return simulate))

(fn `UserConstructionScript`)