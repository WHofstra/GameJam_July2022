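; Enemy character Blueprint that attacks the player on detecting them in range, building on a parent character class.
; It overrides the in-range add and remove functions to accept only BP_PlayerCharacter before passing to the parent.
; An added player triggers PlayerSighted, which uses a short one-shot timer to delay a single Attack call.
; It also supplies its own starting hat count, while a ragdoll physics node sits unconnected.
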(event `self.ReceiveBeginPlay`
  (`parent.ReceiveBeginPlay`))

(event `self.ReceiveActorBeginOverlap`
  (params (OtherActor :type "Actor Object Reference"))
  (`parent.ReceiveActorBeginOverlap` OtherActor))

(event `self.ReceiveTick`
  (params (DeltaSeconds :type "Float (single-precision)"))
  (`parent.ReceiveTick` DeltaSeconds))

(event `PlayerSighted`
  (`KismetSystemLibrary.K2_SetTimerDelegate` (delegate `EnemyAttack`) 0.3))

(event `EnemyAttack`
  (`self.Attack`))

(fn `AddEnemyInRange`
  (params (actor :type "Actor Object Reference (by ref)"))
  (bind _asbp_player_character (cast `/Game/CustomBP/Characters/BP_PlayerCharacter` actor)
    (:`then`
      (`self.PlayerSighted`)
      (`parent.AddEnemyInRange` _asbp_player_character))
    (:`CastFailed`
      _))
  (return))

(fn `GetHatStartAmount`
  (returns (hatAmount :type Integer))
  (return 3))

(fn `RemoveEnemyInRange`
  (params (enemy :type "Actor Object Reference (by ref)"))
  (returns (isRemoved :type Boolean))
  (locals (removed :type Boolean))
  (bind _asbp_player_character (cast `/Game/CustomBP/Characters/BP_PlayerCharacter` enemy)
    (:`then`
      (bind _isremoved (`parent.RemoveEnemyInRange` _asbp_player_character))
      (set `local.removed` _isremoved))
    (:`CastFailed`
      _))
  (return (`local.removed`)))

(fn `UserConstructionScript`
  (`parent.UserConstructionScript`))