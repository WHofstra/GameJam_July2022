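; Custom character Blueprint that picks up hats by touching them and wears them under a Hats component.
; Capsule overlap calls AddHat, which uses BP_HatInterface to check availability, claim the hat and snap-attach it.
; RemoveHat detaches the last attached child, re-enables its availability after a short timer and returns the hat actor.
; The construction script raises jump velocity, and a second capsule overlap event prints debug text.
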(event `self.ReceiveBeginPlay`)

(event `self.ReceiveActorBeginOverlap`
  (params (OtherActor :type "Actor Object Reference")))

(event `self.ReceiveTick`
  (params (DeltaSeconds :type "Float (single-precision)")))

(event `self.CapsuleComponent.OnComponentBeginOverlap`
  (params (OverlappedComponent :type "PrimitiveComponent Object Reference") (OtherActor :type "Actor Object Reference") (OtherComp :type "PrimitiveComponent Object Reference") (OtherBodyIndex :type Integer) (bFromSweep :type Boolean) (SweepResult :type "HitResult Structure (by ref)"))
  (`self.AddHat` OtherActor))

(event `self.Capsule.OnComponentBeginOverlap`
  (params (OverlappedComponent :type "PrimitiveComponent Object Reference") (OtherActor :type "Actor Object Reference") (OtherComp :type "PrimitiveComponent Object Reference") (OtherBodyIndex :type Integer) (bFromSweep :type Boolean) (SweepResult :type "HitResult Structure (by ref)"))
  (`KismetSystemLibrary.PrintString` (`KismetStringLibrary.Concat_StrStr` "'" (`KismetSystemLibrary.GetDisplayName` OtherActor) "' overlap.") true true (struct :`R` 1.0 :`G` 0.919532 :`B` 0.734426 :`A` 1.0) 1.0))

(fn `AddHat`
  (params (hat :type "Actor Object Reference (by ref)"))
  (bind (_oftypehat _hatinterface) (`self.IsOfTypeHat` hat))
  (if _oftypehat
    (bind _isavailable (`/Game/CustomBP/Hats/BP_HatInterface.IsAvailable` _hatinterface))
    (if _isavailable
      (`/Game/CustomBP/Hats/BP_HatInterface.SetAvailabilityTo` _hatinterface false)
      (`self.K2_AttachToComponent` hat (`self.Hats`) "None" "SnapToTarget" "SnapToTarget" "KeepRelative" true))))

(fn `DoesHeadContainHats`
  (returns (containsHats :type Boolean) (hats :type "Array of SceneComponent Object Reference"))
  (bind _hats (`self.GetHats`))
  (return (> (`KismetArrayLibrary.Array_Length` _hats) 0) _hats))

(fn `GetHats`
  (returns (hats :type "Array of SceneComponent Object Reference"))
  (return (`SceneComponent.GetChildrenComponents` (`self.Hats`) false)))

(fn `GetHatStartAmount`
  (returns (hatAmount :type Integer))
  (return 5))

(fn `GetLastSceneComponent`
  (params (sceneComponents :type "Array of SceneComponent Object Reference"))
  (returns (lastComponent :type "SceneComponent Object Reference"))
  (locals (newLastComp :type "SceneComponent Object Reference"))
  (bind _returnvalue (`KismetArrayLibrary.Array_Length` sceneComponents))
  (if (> _returnvalue 0)
    (set `local.newLastComp` (`|GetArrayItem` sceneComponents (- _returnvalue 1))))
  (return (`local.newLastComp`)))

(fn `GetPrimitiveComponent`
  (params (sceneComponent :type "SceneComponent Object Reference (by ref)"))
  (returns (primitiveComponent :type "PrimitiveComponent Object Reference"))
  (locals (primitiveComp :type "PrimitiveComponent Object Reference"))
  (for _array_element (`SceneComponent.GetChildrenComponents` sceneComponent true)
    (bind (_asprimitive_component _bsuccess) (cast `PrimitiveComponent` _array_element :!pure true))
    (if _bsuccess
      (set `local.primitiveComp` _asprimitive_component)
      (break)))
  (return (`local.primitiveComp`)))

(fn `IsOfTypeHat`
  (params (object :type "Actor Object Reference (by ref)"))
  (returns (ofTypeHat :type Boolean) (hatInterface :type "/Game/CustomBP/Hats/BP_HatInterface Interface"))
  (locals (isOfTypeHat :type Boolean) (interface :type "/Game/CustomBP/Hats/BP_HatInterface Interface"))
  (bind _asbp_hat_interface (cast `/Game/CustomBP/Hats/BP_HatInterface` object)
    (:`then`
      (set `local.isOfTypeHat` true)
      (set `local.interface` _asbp_hat_interface))
    (:`CastFailed`
      (set `local.isOfTypeHat` false)))
  (return (`local.isOfTypeHat`) (`local.interface`)))

(fn `RemoveHat`
  (returns (lastHat :type "Actor Object Reference"))
  (bind _hats (`self.GetHats`))
  (bind _lastcomponent (`self.GetLastSceneComponent` _hats))
  (`/Engine/EditorBlueprintResources/StandardMacros.IsValid` _lastcomponent
    (:`Is Valid`
      (`SceneComponent.K2_DetachFromComponent` _lastcomponent "KeepWorld" "KeepWorld" "KeepRelative" true)
      (`|ExecutionSequence`
        (:`then_0`
          (bind _returnvalue (`ActorComponent.GetOwner` _lastcomponent))
          (bind (_asbp_hat_interface _bsuccess) (cast `/Game/CustomBP/Hats/BP_HatInterface` _returnvalue :!pure true))
          (if (and (`KismetSystemLibrary.IsValid` _returnvalue) _bsuccess)
            (`/Game/CustomBP/Hats/BP_HatInterface.SetAvailabilityWithTimer` _asbp_hat_interface true 1.0)))
        (:`then_1`
          (if _bsuccess
            _))
        (:`then_2`
          (return _returnvalue))))))

(fn `UserConstructionScript`
  (`parent.UserConstructionScript`)
  (set `CharacterMovementComponent.JumpZVelocity` 750.0 (`self.CharacterMovement`)))