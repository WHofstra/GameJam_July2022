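; Character that stacks hats on its head and steals them from other characters by kicking.
; Capsule overlap claims available hats through BP_HatInterface, offsetting each by stack height, while a Box overlap tracks BP_CustomCharacter targets in range.
; Attack hurts every tracked target on a timed cooldown with a kick animation.
; A hurt character hands its top hat to the attacker, or is destroyed if it has none.
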(event `self.ReceiveBeginPlay`)

(event `self.ReceiveActorBeginOverlap`
  (params (OtherActor :type "Actor Object Reference")))

(event `self.ReceiveTick`
  (params (DeltaSeconds :type "Float (single-precision)")))

(event `self.CapsuleComponent.OnComponentBeginOverlap`
  (params (OverlappedComponent :type "PrimitiveComponent Object Reference") (OtherActor :type "Actor Object Reference") (OtherComp :type "PrimitiveComponent Object Reference") (OtherBodyIndex :type Integer) (bFromSweep :type Boolean) (SweepResult :type "HitResult Structure (by ref)"))
  (`self.AddHat` OtherActor))

(event `Attack`
  (if (not (`self.hasAttackCooldown`))
    (for _array_element (`self.enemies`)
      (`self.GetHurt` _array_element self))
    (set `self.hasAttackCooldown` true)
    (`KismetSystemLibrary.K2_SetTimerDelegate` (delegate `AttackCooldown`) 0.6)
    (`SkeletalMeshComponent.PlayAnimation` (`self.Mesh`) "/Game/Art/07_Aramature/M_karakter_Rig_Anim_ROBO_Kick.M_karakter_Rig_Anim_ROBO_Kick" false)))

(event `AttackCooldown`
  (set `self.hasAttackCooldown` false)
  (`SkeletalMeshComponent.SetAnimationMode` (`self.Mesh`) "AnimationBlueprint"))

(event `GetHurt`
  (params (attacker :type "/Game/CustomBP/Characters/BP_CustomCharacter Object Reference"))
  (bind _lasthat (`self.RemoveHat`))
  (`self.AddHat` attacker _lasthat))

(event `self.Box.OnComponentBeginOverlap`
  (params (OverlappedComponent :type "PrimitiveComponent Object Reference") (OtherActor :type "Actor Object Reference") (OtherComp :type "PrimitiveComponent Object Reference") (OtherBodyIndex :type Integer) (bFromSweep :type Boolean) (SweepResult :type "HitResult Structure (by ref)"))
  (`self.AddEnemyInRange` OtherActor))

(event `self.Box.OnComponentEndOverlap`
  (params (OverlappedComponent :type "PrimitiveComponent Object Reference") (OtherActor :type "Actor Object Reference") (OtherComp :type "PrimitiveComponent Object Reference") (OtherBodyIndex :type Integer))
  (`self.RemoveEnemyInRange` OtherActor))

(fn `AddEnemyInRange`
  (params (actor :type "Actor Object Reference (by ref)"))
  (bind (_asbp_custom_character _bsuccess) (cast `/Game/CustomBP/Characters/BP_CustomCharacter` actor :!pure true))
  (if _bsuccess
    (`KismetArrayLibrary.Array_Add` (`self.enemies`) _asbp_custom_character)))

(fn `AddHat`
  (params (hat :type "Actor Object Reference (by ref)"))
  (bind _returnvalue (`KismetMathLibrary.Conv_IntToDouble` (`self.hatHeightIndex`)))
  (bind (_oftypehat _hatinterface) (`self.IsOfTypeHat` hat))
  (if _oftypehat
    (bind _isavailable (`/Game/CustomBP/Hats/BP_HatInterface.IsAvailable` _hatinterface))
    (if _isavailable
      (`/Game/CustomBP/Hats/BP_HatInterface.SetAvailabilityTo` _hatinterface false)
      (`self.K2_AttachToComponent` hat (`self.Hats`) "None" "SnapToTarget" "SnapToTarget" "KeepRelative" true)
      (`self.K2_SetActorLocation` hat (+ (`self.K2_GetActorLocation` hat) (* (`self.hatOffset`) (`KismetMathLibrary.MakeVector` _returnvalue _returnvalue _returnvalue))) false true)
      (`/Engine/EditorBlueprintResources/StandardMacros.IncrementInt` (`self.hatHeightIndex`)))))

(fn `CanJumpInternal`
  (returns (ReturnValue :type Boolean))
  (return false))

(fn `DoesHeadContainHats`
  (returns (containsHats :type Boolean) (hats :type "Array of SceneComponent Object Reference"))
  (bind _hats (`self.GetHats`))
  (return (> (`KismetArrayLibrary.Array_Length` _hats) 0) _hats))

(fn `GetHats`
  (returns (hats :type "Array of SceneComponent Object Reference"))
  (return (`SceneComponent.GetChildrenComponents` (`self.Hats`) false)))

(fn `GetHatStartAmount`
  (returns (hatAmount :type Integer))
  (return 5))

(fn `GetLastSceneComponent`
  (params (sceneComponents :type "Array of SceneComponent Object Reference"))
  (returns (lastComponent :type "SceneComponent Object Reference"))
  (locals (newLastComp :type "SceneComponent Object Reference"))
  (bind _returnvalue (`KismetArrayLibrary.Array_Length` sceneComponents))
  (if (> _returnvalue 0)
    (set `local.newLastComp` (`|GetArrayItem` sceneComponents (- _returnvalue 1))))
  (return (`local.newLastComp`)))

(fn `GetPrimitiveComponent`
  (params (sceneComponent :type "SceneComponent Object Reference (by ref)"))
  (returns (primitiveComponent :type "PrimitiveComponent Object Reference"))
  (locals (primitiveComp :type "PrimitiveComponent Object Reference"))
  (for _array_element (`SceneComponent.GetChildrenComponents` sceneComponent true)
    (bind (_asprimitive_component _bsuccess) (cast `PrimitiveComponent` _array_element :!pure true))
    (if _bsuccess
      (set `local.primitiveComp` _asprimitive_component)
      (break)))
  (return (`local.primitiveComp`)))

(fn `IsOfTypeHat`
  (params (object :type "Actor Object Reference (by ref)"))
  (returns (ofTypeHat :type Boolean) (hatInterface :type "/Game/CustomBP/Hats/BP_HatInterface Interface"))
  (locals (isOfTypeHat :type Boolean) (interface :type "/Game/CustomBP/Hats/BP_HatInterface Interface"))
  (bind _asbp_hat_interface (cast `/Game/CustomBP/Hats/BP_HatInterface` object)
    (:`then`
      (set `local.isOfTypeHat` true)
      (set `local.interface` _asbp_hat_interface))
    (:`CastFailed`
      (set `local.isOfTypeHat` false)))
  (return (`local.isOfTypeHat`) (`local.interface`)))

(fn `RemoveEnemyInRange`
  (params (enemy :type "Actor Object Reference (by ref)"))
  (returns (isRemoved :type Boolean))
  (locals (removed :type Boolean))
  (bind (_asbp_custom_character _bsuccess) (cast `/Game/CustomBP/Characters/BP_CustomCharacter` enemy :!pure true))
  (bind _enemies (`self.enemies`))
  (if (and _bsuccess (`KismetArrayLibrary.Array_Contains` _enemies _asbp_custom_character))
    (bind _returnvalue (`KismetArrayLibrary.Array_RemoveItem` _enemies _asbp_custom_character))
    (set `local.removed` _returnvalue))
  (return (`local.removed`)))

(fn `RemoveHat`
  (returns (lastHat :type "Actor Object Reference"))
  (bind _hats (`self.GetHats`))
  (bind _lastcomponent (`self.GetLastSceneComponent` _hats))
  (`/Engine/EditorBlueprintResources/StandardMacros.IsValid` _lastcomponent
    (:`Is Valid`
      (`SceneComponent.K2_DetachFromComponent` _lastcomponent "KeepWorld" "KeepWorld" "KeepRelative" true)
      (`|ExecutionSequence`
        (:`then_0`
          (bind _returnvalue (`ActorComponent.GetOwner` _lastcomponent))
          (bind (_asbp_hat_interface _bsuccess) (cast `/Game/CustomBP/Hats/BP_HatInterface` _returnvalue :!pure true))
          (if (and (`KismetSystemLibrary.IsValid` _returnvalue) _bsuccess)
            (`/Game/CustomBP/Hats/BP_HatInterface.SetAvailabilityTo` _asbp_hat_interface true)))
        (:`then_1`
          (`/Engine/EditorBlueprintResources/StandardMacros.DecrementInt` (`self.hatHeightIndex`)
            (:`  `
              (return _returnvalue))))))
    (:`Is Not Valid`
      (`self.K2_DestroyActor`))))

(fn `UserConstructionScript`
  (`parent.UserConstructionScript`)
  (set `CharacterMovementComponent.JumpZVelocity` 750.0 (`self.CharacterMovement`)))