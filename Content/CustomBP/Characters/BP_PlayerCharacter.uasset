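; Player character Blueprint that specializes a parent character class and sends the game back to the title screen on death.
; Overrides of the add and remove enemy-in-range functions pass only BP_EnemyCharacter actors on to the parent logic.
; Die calls ActivateDeath, and a separate DeathEvent loads the TitleScreen level.
; BeginPlay, overlap, Tick and construction simply defer to the parent.
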(event `self.ReceiveBeginPlay`
  (`parent.ReceiveBeginPlay`))

(event `self.ReceiveActorBeginOverlap`
  (params (OtherActor :type "Actor Object Reference"))
  (`parent.ReceiveActorBeginOverlap` OtherActor))

(event `self.ReceiveTick`
  (params (DeltaSeconds :type "Float (single-precision)"))
  (`parent.ReceiveTick` DeltaSeconds))

(event `self.DeathEvent`
  (`GameplayStatics.OpenLevel` "TitleScreen"))

(fn `AddEnemyInRange`
  (params (actor :type "Actor Object Reference (by ref)"))
  (bind _asbp_enemy_character (cast `/Game/CustomBP/Characters/BP_EnemyCharacter` actor)
    (:`then`
      (`parent.AddEnemyInRange` _asbp_enemy_character))
    (:`CastFailed`
      _))
  (return))

(fn `Die`
  (`self.ActivateDeath` 0.5))

(fn `RemoveEnemyInRange`
  (params (enemy :type "Actor Object Reference (by ref)"))
  (returns (isRemoved :type Boolean))
  (locals (removed :type Boolean))
  (bind _asbp_enemy_character (cast `/Game/CustomBP/Characters/BP_EnemyCharacter` enemy)
    (:`then`
      (bind _isremoved (`parent.RemoveEnemyInRange` _asbp_enemy_character))
      (set `local.removed` _isremoved))
    (:`CastFailed`
      _))
  (return (`local.removed`)))

(fn `UserConstructionScript`
  (`parent.UserConstructionScript`))