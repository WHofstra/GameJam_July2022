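; BP_HatSpawnerComponent is a component that spawns hat objects with a randomly chosen model.
; CreateHat spawns a BP_TestObject at a given transform, adjusting for collisions, and sets its static mesh to a random entry from HatModelArray.
; CreateHatWithCharacter calls CreateHat at a character's transform, raised above its location, and returns the new hat without attaching it.
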(event `self.ReceiveBeginPlay`)

(event `self.ReceiveTick`
  (params (DeltaSeconds :type "Float (single-precision)")))

(fn `CreateHat`
  (params (transform :type "Transform Structure"))
  (returns (newHat :type "/Game/CustomBP/TestMDL/BP_TestObject Object Reference"))
  (locals (stream :type "RandomStream Structure" :default (struct :`InitialSeed` 29980)))
  (bind _returnvalue (`|SpawnActorFromClass` "/Game/CustomBP/TestMDL/BP_TestObject.BP_TestObject_C" transform "AdjustIfPossibleButAlwaysSpawn" "OverrideRootScale" null null))
  (`StaticMeshComponent.SetStaticMesh` (`/Game/CustomBP/TestMDL/BP_TestObject.StaticMesh` _returnvalue) (`KismetArrayLibrary.Array_Random` (`self.hatModelArray`)))
  (return _returnvalue))

(fn `CreateHatWithCharacter`
  (params (character :type "/Game/CustomBP/Characters/BP_CustomCharacter Object Reference"))
  (returns (newHat :type "/Game/CustomBP/TestMDL/BP_TestObject Object Reference"))
  (bind (_returnvalue_location _returnvalue_rotation _returnvalue_scale) (`KismetMathLibrary.BreakTransform` (`Actor.GetTransform` character)))
  (bind _newhat (`self.CreateHat` (`KismetMathLibrary.MakeTransform` (+ _returnvalue_location (0.0 0.0 75.0)) _returnvalue_rotation _returnvalue_scale)))
  (return _newhat))